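; Final dungeon door that swings open its two large leaves when interacted with, provided the KeyInventory flag on KeyTaken is set.
; The Interaction event checks that flag, plays the door-open sound at the actor's location and starts a timeline.
; Each update sets the left and right leaves' relative yaw in opposite directions through Lerps that take the track as A and ±90 as Alpha, so they extrapolate rather than blend.
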(event EventBeginPlay)

(event Collision|EventActorBeginOverlap
  (params (OtherActor :type Actor%20Object%20Reference)))

(event EventTick
  (params (DeltaSeconds :type Float%20%28single-precision%29)))

(event EventInteraction
  (if (Variables|/Game/MedievalDungeon/Blueprints/SM_Lock_Key3_Blueprint.SM_Lock_Key3_Blueprint_C|GetKey%20Inventory (Variables|Default|GetKeyTaken))
    (Audio|PlaySoundatLocation "/Game/Audio/SFX_Door_Open.SFX_Door_Open" (Transformation|GetActorLocation) "0, 0, 0" 1.0 1.0 0.0 0 0 0 0)
    (bind _newtrack_0 (Timeline|Timeline Play)
      (:Update
        (Transformation|SetRelativeRotation (Variables|Default|GetSM_DoorWay_Large_Door_Left) (Math|Rotator|MakeRotator 0.0 0.0 (Math|Float|Lerp _newtrack_0 0.0 -9e+01)) false false)
        (Transformation|SetRelativeRotation (Variables|Default|GetSM_DoorWay_Large_Door_Right) (Math|Rotator|MakeRotator 0.0 0.0 (Math|Float|Lerp _newtrack_0 0.0 9e+01)) false false)))))

(fn ConstructionScript)